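; Elizabeth enemy Blueprint that implements a charge attack, ramming through the level until it hits something.
; Beginning a charge disables manual target facing and multiplies movement speed through a multicast; ending it reverses both and signals that the charge has ended.
; While charging, capsule hits ignore projectiles; any other hit ends the charge, destroying treasure chests and dealing armor-piercing damage to player characters.
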(event `Begin Charging`
  (`self.SetManuallyFaceTarget` false)
  (`self.Multicast_SetMovementSpeed` (* (`MovementComponent.GetMaxSpeed` (`self.GetMovementComponent`)) 4.0))
  (set `self.Charging` true))

(event `End Charging`
  (`self.Multicast_SetMovementSpeed` (/ (`MovementComponent.GetMaxSpeed` (`self.GetMovementComponent`)) 4.0))
  (set `self.Charging` false)
  (`self.ChargeEnded`)
  (`self.SetManuallyFaceTarget` true))

(event `self.CapsuleComponent.OnComponentHit`
  (params (HitComponent :type "PrimitiveComponent Object Reference") (OtherActor :type "Actor Object Reference") (OtherComp :type "PrimitiveComponent Object Reference") (NormalImpulse :type "Vector Structure") (Hit :type "HitResult Structure (by ref)"))
  (if (`self.Charging`)
    (cast `Projectile` OtherActor
      (:`CastFailed`
        (bind _asbp_treasure_chest (cast `/Game/Core/BP_TreasureChest` _)
          (:`then`
            (`/Game/Core/BP_TreasureChest.DestroyChest` _asbp_treasure_chest))
          (:`CastFailed`
            _))
        (`self.End Charging`)
        (bind _aspirate_survivors_character (cast `PirateSurvivorsCharacter` OtherActor))
        (`HealthComponent.TakeDamage` (`self.GetHealthComponent` _aspirate_survivors_character) (make `DamageInstance` "Elizabeth's Charge" 40.0 true self))))))

(fn `UserConstructionScript`)