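; BP_TreasureChest is an interactable chest that bursts into XP pickups when opened, then disappears.
; Interaction on the authority calls OpenChest, which removes the interaction components, rotates the lid by timeline, then spawns randomized physics XP through the game state's XPManager.
; After a delay, or directly via DestroyChest, it scales away, fires ChestDestroyed and destroys itself.
; The same scale timeline plays reversed on BeginPlay, with a Destroyed flag preventing premature destruction.
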(event `OpenChest`
  (`ActorComponent.K2_DestroyComponent` (`InteractableComponent.InteractionRange` (`self.Interactable`)))
  (`ActorComponent.K2_DestroyComponent` (`self.Interactable`))
  (bind (_direction _pitch) (`Timeline|OpenTimeline`)
    (:`Update`
      (`SceneComponent.K2_SetRelativeRotation` (`self.Lid`) (`KismetMathLibrary.MakeRotator` 0.0 _pitch) false false))
    (:`Finished`
      (`/Engine/EditorBlueprintResources/ActorMacros.Switch Has Authority`
        (:`Authority`
          (for _ (range (+ (`KismetMathLibrary.RandomIntegerInRange` 15 25) 1))
            (`XPManager.SpawnXPWithPhysics` (`PirateGameState.XPManager` (`PirateGameState.GetPirateGameState`)) (`SceneComponent.K2_GetComponentLocation` (`self.XPSpawnLoc`)) (`KismetMathLibrary.RandomFloatInRange` 1.0 2.5) 0 (`KismetMathLibrary.MakeVector` (`KismetMathLibrary.RandomFloatInRange` -200.0 200.0) (`KismetMathLibrary.RandomFloatInRange` -200.0 200.0) (`KismetMathLibrary.RandomFloatInRange` 0.0 200.0))))
          (`KismetSystemLibrary.Delay` 4.0)
          (set `self.Destroyed` true :!label _label)
          (bind (_direction_2 _scale) (`Timeline|Disappear` :!label _label_2)
            (:`Update`
              (`self.SetActorScale3D` (`KismetMathLibrary.Conv_DoubleToVector` _scale)))
            (:`Finished`
              (if (`self.Destroyed`)
                (`KismetSystemLibrary.Delay` 0.5)
                (`self.ChestDestroyed`)
                (`self.K2_DestroyActor`)))))))))

(event `self.Interactable.OnInteract`
  (params (Interactor :type "PiratePlayerState Object Reference"))
  (`/Engine/EditorBlueprintResources/ActorMacros.Switch Has Authority`
    (:`Authority`
      (`self.OpenChest`))))

(event `DestroyChest`
  (goto _label))

(event `self.ReceiveBeginPlay`
  (goto _label_2 :!via `ReverseFromEnd`))

(fn `UserConstructionScript`)