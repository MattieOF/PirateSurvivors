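; Server-only spawner that places a BP_TreasureChest at its own transform, destroying itself on remote clients.
; A delay-driven loop spawns a chest when none exists and, six seconds later, can randomly despawn it if HasDespawnChance is set.
; If that roll fails the loop stops until the chest's destroyed event clears HasChest and restarts the delay.
; The spawn roll has full weight, so it always passes.
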(event `self.ReceiveBeginPlay`
  (`/Engine/EditorBlueprintResources/ActorMacros.Switch Has Authority`
    (:`Authority`
      (if (`KismetMathLibrary.RandomBoolWithWeight` 1.0) :!label _label
        (if (`self.HasChest`)
          (if (and (`KismetMathLibrary.RandomBoolWithWeight` 0.2) (`self.HasDespawnChance`))
            (`/Game/Core/BP_TreasureChest.DestroyChest` (`self.Chest`))
            (set `self.HasChest` false)
            (`KismetSystemLibrary.Delay` 6.0 :!label _label_2)
            (goto _label))
          (else
            (bind _returnvalue (`|SpawnActorFromClass` "/Game/Core/BP_TreasureChest.BP_TreasureChest_C" (`self.GetTransform`) "Undefined" "MultiplyWithRoot" null null))
            (add `/Game/Core/BP_TreasureChest.ChestDestroyed` _returnvalue (delegate `ChestDestroyed`))
            (set `self.HasChest` true)
            (set `self.Chest` _returnvalue)
            (goto _label_2)))
        (else
          (`KismetSystemLibrary.Delay` 6.0)
          (goto _label))))
    (:`Remote`
      (`self.K2_DestroyActor`))))

(event `ChestDestroyed`
  (set `self.HasChest` false)
  (goto _label_2))

(fn `UserConstructionScript`)