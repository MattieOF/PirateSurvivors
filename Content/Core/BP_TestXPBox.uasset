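; BP_TestXPBox is a test actor that scatters XP pickups inside its box volume when play begins.
; On the server only, it polls every 0.1 seconds until the pirate game state's XP manager is valid.
; It then loops over Count, multicasting spawns at random points in the box, each worth one XP with a free ID from the manager.
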(event `self.ReceiveBeginPlay`
  (bind _box (`self.Box`))
  (`/Engine/EditorBlueprintResources/ActorMacros.Switch Has Authority`
    (:`Authority`
      (`KismetSystemLibrary.Delay` 0.0)
      (`/Engine/EditorBlueprintResources/StandardMacros.IsValid` (`PirateGameState.XPManager` (`PirateGameState.GetPirateGameState`)) :!label _label
        (:`Is Valid`
          (for _ (range (+ (`self.Count`) 1))
            (`XPManager.Multicast_SpawnXP` (`PirateGameState.XPManager` (`PirateGameState.GetPirateGameState`)) (`KismetMathLibrary.RandomPointInBoundingBox` (`SceneComponent.K2_GetComponentLocation` _box) (`BoxComponent.GetScaledBoxExtent` _box)) 1.0 (`XPManager.GetFreeID` (`PirateGameState.XPManager` (`PirateGameState.GetPirateGameState`))))))
        (:`Is Not Valid`
          (`KismetSystemLibrary.Delay` 0.1)
          (goto _label))))))

(fn `UserConstructionScript`)