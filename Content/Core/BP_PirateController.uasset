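; Player controller for the pirate game that builds the local UI and binds a weapon-grant key.
; CreateUI retries each tick until HasLoaded is true, then creates the XP bar and HUD widgets and adds them to the viewport.
; Pressing G, only when running with authority, gives the Cat O' Nine weapon through PiratePlayerState, with no server RPC for clients.
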(event `self.CreateUI`
  (bind _aspirate_player_state (cast `PiratePlayerState` (`self.PlayerState`) :!pure true))
  (if (`self.HasLoaded`) :!label _label
    ;[1 1 1] UI
    (bind _returnvalue (`|CreateWidget` "/Game/UI/W_XPBar.W_XPBar_C" null _aspirate_player_state))
    (`UserWidget.AddToViewport` _returnvalue 0)
    (bind _returnvalue_2 (`|CreateWidget` "/Game/UI/W_HUD.W_HUD_C" null _aspirate_player_state))
    (`UserWidget.AddToViewport` _returnvalue_2 0)
    (else
      (`KismetSystemLibrary.DelayUntilNextTick`)
      (goto _label))))

(event `Key|G`
  (params (Key :type "Key Structure"))
  (:`Pressed`
    (`/Engine/EditorBlueprintResources/ActorMacros.Switch Has Authority`
      (:`Authority`
        (`PiratePlayerState.GiveWeaponFromType` (cast `PiratePlayerState` (`self.PlayerState`) :!pure true) "/Game/Weapons/CatONine/WPN_CatONine.WPN_CatONine")))))

(fn `UserConstructionScript`)