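; Summoned cannon turret that automatically fires cannonballs at nearby enemies on behalf of its owning character.
; Authority-only Tick waits out a fire cooldown, then finds the closest enemy within a range scaled from its Stats.
; It snaps its yaw toward that target and spawns a cannonball projectile from the muzzle offset, aimed directly at the enemy.
; Each shot spends ammo, and the actor destroys itself shortly after the last one.
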(event `self.ReceiveTick`
  (params (DeltaSeconds :type "Float (single-precision)"))
  (bind _returnvalue (+ (`self.K2_GetActorLocation`) (`self.ShootPos`)))
  (bind _returnvalue_2 (`WeaponFunctionality.GetClosestEnemyWithinRange` _returnvalue (* (`WeaponStats.Range` (`self.Stats`)) 7.0)))
  (bind _returnvalue_3 (`KismetMathLibrary.Normal` (- (`self.K2_GetActorLocation` _returnvalue_2) _returnvalue)))
  (bind (_returnvalue_roll _returnvalue_pitch _returnvalue_yaw) (`KismetMathLibrary.BreakRotator` (`KismetMathLibrary.Conv_VectorToRotator` _returnvalue_3)))
  (`/Engine/EditorBlueprintResources/ActorMacros.Switch Has Authority`
    (:`Authority`
      (if (and (<= (`self.FireCooldown`) 0.0) (> (`self.AmmoLeft`) 0))
        (`/Engine/EditorBlueprintResources/StandardMacros.IsValid` _returnvalue_2
          (:`Is Valid`
            (`self.K2_SetActorRotation` (`KismetMathLibrary.MakeRotator` 0.0 0.0 _returnvalue_yaw))
            (`Projectile.SpawnProjectile` (`self.OwningCharacter`) (`self.Stats`) (`KismetMathLibrary.TransformLocation` (`self.GetTransform`) (`self.ShootPos`)) _returnvalue_3 "/Game/Weapons/Cannon/PROJ_Cannonball.PROJ_Cannonball")
            (set `self.FireCooldown` 1.3)
            (bind _result (`/Engine/EditorBlueprintResources/StandardMacros.DecrementInt` (`self.AmmoLeft`))
              (:`  `
                (if (<= _result 0)
                  (`KismetSystemLibrary.Delay` 1.0)
                  (`self.K2_DestroyActor`))))))
        (else
          (set `self.FireCooldown` (- (`self.FireCooldown`) DeltaSeconds)))))))

(fn `UserConstructionScript`)